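; Base Blueprint for fruit collectables in a Paper2D game, picked up when an actor tagged Player overlaps its collision.
; On pickup it disables collision and switches the render component to a non-looping collected flipbook.
; A looping timer then polls the flipbook and destroys the actor once the animation stops playing.
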(event OnComponentBeginOverlap(Collision)
  (params (OverlappedComponent :type Primitive%20Component%20Object%20Reference) (OtherActor :type Actor%20Object%20Reference) (OtherComp :type Primitive%20Component%20Object%20Reference) (OtherBodyIndex :type Integer) (bFromSweep :type Boolean) (SweepResult :type Hit%20Result%20Structure%20%28by%20ref%29))
  ;[0.15 0.15 0.15 0.5] Player collects the fruit
  (if (Actor|ActorHasTag OtherActor "Player")
    ;[0.15 0.15 0.15 0.5] Sequence for collecting fruit
    (Collision|SetCollisionEnabled (Variables|Default|GetCollision) "NoCollision")
    (Sprite|SetFlipbook (Variables|Default|GetRenderComponent) "/Game/Assets/Items/Fruits/Flipbooks/FB_Collected.FB_Collected")
    (Components|Timeline|SetLooping (Variables|Default|GetRenderComponent) false)
    ;[0.15 0.15 0.15 0.5] Check if collect animation is completed, once complete destroy
    (Utilities|Time|SetTimerbyEvent (delegate Custom|TryDestroyItem) 0.15 true)))

(event Custom|TryDestroyItem
  ;[0.15 0.15 0.15 0.5] Check if collect animation is completed, once complete destroy
  (if (not (Audio|Components|Audio|IsPlaying (Variables|Default|GetRenderComponent)))
    (Actor|DestroyActor)))

(fn ConstructionScript)