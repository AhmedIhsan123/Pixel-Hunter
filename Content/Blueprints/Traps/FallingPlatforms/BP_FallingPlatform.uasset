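; BP_FallingPlatform is a trap platform that bounces and then falls away when the player lands on top of it.
; Its trigger box overlap checks for the Player tag, then Platform Logic uses the hit's impact normal Z to confirm a top hit, store the start location and remove the trigger.
; Chained timelines lerp the platform through a small downward bounce, then a long drop that ends with the actor destroying itself.
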(event OnComponentBeginOverlap(TriggerBox)
  (params (OverlappedComponent :type Primitive%20Component%20Object%20Reference) (OtherActor :type Actor%20Object%20Reference) (OtherComp :type Primitive%20Component%20Object%20Reference) (OtherBodyIndex :type Integer) (bFromSweep :type Boolean) (SweepResult :type Hit%20Result%20Structure%20%28by%20ref%29))
  ;[0.15 0.15 0.15 0.5] Listen for overlap events and trigger platform logic based on player hit
  ;;[0.15 0.15 0.15 0.5] Check for player tag
  (if (Actor|ActorHasTag OtherActor "Player")
    (|PlatformLogic SweepResult)))

(fn ConstructionScript)