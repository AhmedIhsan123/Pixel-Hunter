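; BP_PlayerBase is a 2D side-scrolling player character with Enhanced Input movement along X, jumping, double jump and coyote time.
; Each tick it picks an idle, run, jump, fall or double-jump flipbook from velocity and jump count, and turns the controller to face travel direction.
; Walking off a ledge opens a brief timed window where jumping raises the jump limit once, and landing resets it.
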(event EventBeginPlay
  ;[0.15 0.15 0.15 0.5] Event begin play
  ;;[0.15 0.15 0.15 0.5] Add player input mapping context
  (Input|AddMappingContext (PlayerController|LocalPlayerSubsystems|GetEnhancedInputLocalPlayerSubsystem (Game|GetPlayerController 0)) "/Game/Blueprints/Characters/Input/IMC_PlayerInput.IMC_PlayerInput" 0 "(bIgnoreAllPressedKeysUntilRelease=True,bForceImmediately=False,bNotifyUserSettings=False)"))

(event EventTick
  (params (DeltaSeconds :type Float%20%28single-precision%29))
  ;[0.15 0.15 0.15 0.5] Event tick
  (Character|UpdatePlayerState))

(event EventOnMovementModeChanged
  (params (PrevMovementMode :type EMovementMode%20Enum :default "MOVE_None") (NewMovementMode :type EMovementMode%20Enum :default "MOVE_None") (PrevCustomMode :type Byte :default 0) (NewCustomMode :type Byte :default 0))
  ;[0.15 0.15 0.15 0.5] Coyote time
  (|CoyoteTime PrevMovementMode NewMovementMode))

(fn ConstructionScript)

(fn UpdatePlayerState
  (bind _returnvalue (Game|GetPlayerController 0))
  ;[0.15 0.15 0.15 0.5] Update the players state
  (Utilities|FlowControl|Sequence
    (:then_0
      (Animation|UpdatePlayerAnimation))
    (:then_1
      ;;[0.15 0.15 0.15 0.5] Update player rotation
      (Math|Float|CompareFloat (.x (Transformation|GetVelocity)) 0.0
        (:>
          (Pawn|SetControlRotation _returnvalue (Math|Rotator|MakeRotator 0.0 0.0 0.0)))
        (:<
          (Pawn|SetControlRotation _returnvalue (Math|Rotator|MakeRotator 0.0 0.0 1.8e+02)))))))

(fn UpdatePlayerAnimation
  (params (IdleAnim :type Paper%20Flipbook%20Object%20Reference) (RunAnim :type Paper%20Flipbook%20Object%20Reference) (JumpAnim :type Paper%20Flipbook%20Object%20Reference) (FallAnim :type Paper%20Flipbook%20Object%20Reference) (DoubleJumpAnim :type Paper%20Flipbook%20Object%20Reference))
  ;[0.15 0.15 0.15 0.5] Update animation
  (Variables|Animation|SetAnimationState (select (> (Math|Vector|VectorLength (Transformation|GetVelocity)) 0.0) (select (AI|Components|NavMovement|IsFalling (Variables|Character|GetCharacterMovement)) (select (< (.z (Transformation|GetVelocity)) 0.0) "NewEnumerator4" (select (select (> (Variables|Default|GetJumpMaxCount) 2) (> (Variables|Default|GetJumpCurrentCount) 2) (> (Variables|Default|GetJumpCurrentCount) 1)) "NewEnumerator6" "NewEnumerator3")) "NewEnumerator2") "NewEnumerator1"))
  ;;[0.15 0.15 0.15 0.5] Set animation flipbook
  (Sprite|SetFlipbook (Variables|Default|GetSprite) (Utilities|Select :Index (Variables|Animation|GetAnimationState) :NewEnumerator0 0 :NewEnumerator1 IdleAnim :NewEnumerator2 RunAnim :NewEnumerator3 JumpAnim :NewEnumerator4 FallAnim :NewEnumerator6 DoubleJumpAnim)))

(fn DisableCoyoteTime
  (Variables|CoyoteTime|SetbCanUseCoyoteTime false))

(fn CanJumpInternal
  ;[0.15 0.15 0.15 0.5] Can jump + coyote time
  (return (< (Variables|Default|GetJumpCurrentCount) (Variables|Default|GetJumpMaxCount))))

(event Custom|ResetJump
  ;[0.15 0.15 0.15 0.5] Player jump input
  (Utilities|FlowControl|DoOnce false) ; enters at Reset
)

(event Input|EnhancedActionEvents|EnhancedInputActionIA_PlayerMove
  (params (ActionValue :type Float%20%28double-precision%29) (ElapsedSeconds :type Float%20%28double-precision%29) (TriggeredSeconds :type Float%20%28double-precision%29) (InputAction :type Input%20Action%20Object%20Reference :default "/Game/Blueprints/Characters/Input/Actions/IA_PlayerMove.IA_PlayerMove"))
  ;[0.15 0.15 0.15 0.5] Player move input
  (Pawn|Input|AddMovementInput "1.000000,0.000000,0.000000" ActionValue false))

(event Input|EnhancedActionEvents|EnhancedInputActionIA_PlayerJump
  (params (ActionValue :type Boolean) (ElapsedSeconds :type Float%20%28double-precision%29) (TriggeredSeconds :type Float%20%28double-precision%29) (InputAction :type Input%20Action%20Object%20Reference :default "/Game/Blueprints/Characters/Input/Actions/IA_PlayerJump.IA_PlayerJump"))
  ;[0.15 0.15 0.15 0.5] Player jump input
  (if (Variables|CoyoteTime|GetbCanUseCoyoteTime)
    (Utilities|FlowControl|DoOnce false
      (:Completed
        (Variables|Default|SetJumpMaxCount 3)
        (Character|Jump)))
    (else
      (Character|Jump))))

(event EventOnLanded
  (params (Hit :type Hit%20Result%20Structure%20%28by%20ref%29))
  ;[0.15 0.15 0.15 0.5] Clear timer and disable coyote time on land
  (Variables|CoyoteTime|SetbCanUseCoyoteTime false)
  (Utilities|Time|ClearandInvalidateTimerbyHandle (Variables|CoyoteTime|GetCoyoteTimer))
  (CallFunction|ResetJump)
  (Variables|Default|SetJumpMaxCount 2))